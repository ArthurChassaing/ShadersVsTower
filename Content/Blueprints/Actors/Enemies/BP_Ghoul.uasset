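; BP_Ghoul is an enemy character with health, a 3D health bar and death handling.
; Incoming damage is forwarded to a damageable component, whose events update the child-actor health bar and trigger death.
; On death it stops moving, plays a sound and ignores all capsule collision.
; Tick tracks an IsMoving flag from velocity, and Range overlaps are passed to tower in-range and out-of-range handlers.
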(event `self.ReceiveBeginPlay`
  ;[1 1 1] Init event + health bar
  (add `self.OnTakeAnyDamage` (delegate `OnTakeAnyDamage_Event`))
  (bind _asbp_health_bar_3d (cast `/Game/Blueprints/Actors/BP_HealthBar3D` (`ChildActorComponent.ChildActor` (`self.ChildActor`))))
  (set `self.HealthBar` _asbp_health_bar_3d))

(event `OnTakeAnyDamage_Event` :!signature `self.OnTakeAnyDamage`
  (params (DamagedActor :type "Actor Object Reference") (Damage :type "Float (single-precision)") (DamageType :type "DamageType Object Reference") (InstigatedBy :type "Controller Object Reference") (DamageCauser :type "Actor Object Reference"))
  ;[1 1 1] Take damage
  (`/Game/Blueprints/Components/BP_Damageable.Damage` (`self.BP_Damageable`) Damage))

(event `self.BP_Damageable.TakeDamage`
  (params (NewHealth :type "Float (double-precision)") (MaxHealth :type "Float (double-precision)"))
  ;[1 1 1] Take damage
  (`/Game/Blueprints/Actors/BP_HealthBar3D.UpdateHeathPercentage` (`self.HealthBar`) NewHealth MaxHealth))

(event `self.ReceiveTick`
  (params (DeltaSeconds :type "Float (single-precision)"))
  (set `self.IsMoving` (> (`KismetMathLibrary.VSize` (`MovementComponent.Velocity` (`self.CharacterMovement`))) 0.1)))

(event `self.BP_Damageable.OnDie`
  ;[1 1 1] Die!!!!!!!!!!!!!!!!!!!!!!!!!
  (set `self.IsDead` true)
  (`MovementComponent.StopMovementImmediately` (`self.CharacterMovement`))
  (`GameplayStatics.PlaySoundAtLocation` "/Game/Audio/Death_Ghoul.Death_Ghoul" (`self.K2_GetActorLocation`) (struct) 1.0 1.0 0.0 null null null null)
  (`PrimitiveComponent.SetCollisionResponseToAllChannels` (`self.CapsuleComponent`) "ECR_Ignore"))

(event `self.Range.OnComponentBeginOverlap`
  (params (OverlappedComponent :type "PrimitiveComponent Object Reference") (OtherActor :type "Actor Object Reference") (OtherComp :type "PrimitiveComponent Object Reference") (OtherBodyIndex :type Integer) (bFromSweep :type Boolean) (SweepResult :type "HitResult Structure (by ref)"))
  ;[1 1 1] Tower in range
  (`self.OnTowerInRange` OtherActor))

(event `self.Range.OnComponentEndOverlap`
  (params (OverlappedComponent :type "PrimitiveComponent Object Reference") (OtherActor :type "Actor Object Reference") (OtherComp :type "PrimitiveComponent Object Reference") (OtherBodyIndex :type Integer))
  ;[1 1 1] Tower in range
  (`self.OnTowerOutOfRange` OtherActor))

(fn `UserConstructionScript`)