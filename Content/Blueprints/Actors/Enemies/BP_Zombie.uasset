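; BP_Zombie is an enemy zombie character that takes damage, shows a 3D health bar and dies.
; Incoming damage passes to a damageable component, whose callbacks update the bar, briefly flag a hit reaction, or on death detach the controller, disable collision and play a sound.
; Tick derives a moving flag from velocity.
; A range component forwards overlaps as tower in-range and out-of-range notifications; the Attacc function is an empty stub.
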(event `self.ReceiveBeginPlay`
  ;[1 1 1] Init events + health bar
  (bind _asbp_health_bar_3d (cast `/Game/Blueprints/Actors/BP_HealthBar3D` (`ChildActorComponent.ChildActor` (`self.HealthBar`))))
  (set `self.HPBar` _asbp_health_bar_3d)
  (add `self.OnTakeAnyDamage` (delegate `OnTakeAnyDamage_Event`)))

(event `OnTakeAnyDamage_Event` :!signature `self.OnTakeAnyDamage`
  (params (DamagedActor :type "Actor Object Reference") (Damage :type "Float (single-precision)") (DamageType :type "DamageType Object Reference") (InstigatedBy :type "Controller Object Reference") (DamageCauser :type "Actor Object Reference"))
  ;[1 1 1] Got hit
  (`/Game/Blueprints/Components/BP_Damageable.Damage` (`self.BP_Damageable`) Damage))

(event `self.BP_Damageable.TakeDamage`
  (params (NewHealth :type "Float (double-precision)") (MaxHealth :type "Float (double-precision)"))
  ;[1 1 1] Got hit
  (`/Game/Blueprints/Actors/BP_HealthBar3D.UpdateHeathPercentage` (`self.HPBar`) NewHealth MaxHealth)
  (set `self.IsTakingDamage` true)
  (`KismetSystemLibrary.Delay` 0.5)
  (set `self.IsTakingDamage` false))

(event `self.BP_Damageable.OnDie`
  ;[1 1 1] Die!!!!!!!!!!!!!!!!!!!!!!!!!!!!!!!!!!!!!!
  (`self.DetachFromControllerPendingDestroy`)
  (`PrimitiveComponent.SetCollisionResponseToAllChannels` (`self.CapsuleComponent`) "ECR_Ignore")
  (set `self.IsDead` true)
  (`GameplayStatics.PlaySoundAtLocation` null (`self.K2_GetActorLocation`) (struct) 1.0 1.0 0.0 null null null null))

(event `self.ReceiveTick`
  (params (DeltaSeconds :type "Float (single-precision)"))
  (set `self.IsMoving` (> (`KismetMathLibrary.VSize` (`MovementComponent.Velocity` (`self.CharacterMovement`))) 0.1)))

(event `self.Range.OnComponentBeginOverlap`
  (params (OverlappedComponent :type "PrimitiveComponent Object Reference") (OtherActor :type "Actor Object Reference") (OtherComp :type "PrimitiveComponent Object Reference") (OtherBodyIndex :type Integer) (bFromSweep :type Boolean) (SweepResult :type "HitResult Structure (by ref)"))
  ;[1 1 1] Tower in range
  (`self.OnTowerInRange` OtherActor))

(event `self.Range.OnComponentEndOverlap`
  (params (OverlappedComponent :type "PrimitiveComponent Object Reference") (OtherActor :type "Actor Object Reference") (OtherComp :type "PrimitiveComponent Object Reference") (OtherBodyIndex :type Integer))
  ;[1 1 1] Tower in range
  (`self.OnTowerOutOfRange` OtherComp))

(fn `Attacc`)

(fn `UserConstructionScript`)