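; BP_Enemy is an enemy character that stops to melee-attack towers in range.
; OnTowerInRange stores the tower, sets IsAttacking and halts movement, while OnTowerOutOfRange clears that flag but keeps the reference.
; TryDoMeleeDamage passes Damage to the stored tower's BPDamageable if the tower is valid, and NukeEnemy destroys the enemy.
; The event graph is empty, so these functions are not triggered within this Blueprint.
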(fn `NukeEnemy`
  (`self.K2_DestroyActor`))

(fn `OnTowerInRange`
  (params (Object :type "Object Object Reference"))
  (bind _asbp_tower (cast `/Game/Blueprints/Actors/Map/BP_Tower` Object))
  (set `self.IsAttacking` true)
  (set `self.TowerRef` _asbp_tower)
  (`MovementComponent.StopMovementImmediately` (`self.CharacterMovement`)))

(fn `OnTowerOutOfRange`
  (params (Object :type "Object Object Reference"))
  (cast `/Game/Blueprints/Actors/Map/BP_Tower` Object)
  (set `self.IsAttacking` false))

(fn `TryDoMeleeDamage`
  (bind _towerref (`self.TowerRef`)
    (:`then`
      (`/Game/Blueprints/Components/BP_Damageable.Damage` (`.BP_Damageable` (`/Game/Blueprints/Actors/Map/BP_Tower.BP_Damageable` _towerref)) (`self.Damage`)))
    (:`else`)))

(fn `UserConstructionScript`)