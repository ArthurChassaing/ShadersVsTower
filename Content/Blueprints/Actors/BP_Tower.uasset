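; BP_Tower is a destructible turret that fires at the player while a BP_Hero is inside its range.
; Range overlap starts and clears a looping timer that spawns a BP_BigProjectile at the Fire point and impulses it toward player character 0.
; Any damage lowers CurrentLife, updates the WBP_TowerHUD health bar and destroys the tower at zero.
; Tick rotates the health bar widget to face the player camera.
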(event `self.ReceiveBeginPlay`
  (set `self.CurrentLife` (`self.MaxLife`)))

(event `self.ReceiveTick`
  (params (DeltaSeconds :type "Float (single-precision)"))
  (bind _healthbarwidget (`self.HealthBarWidget`))
  ;[1 1 1] Set rotation of health bar
  (`SceneComponent.K2_SetWorldRotation` _healthbarwidget (`KismetMathLibrary.FindLookAtRotation` (`SceneComponent.K2_GetComponentLocation` _healthbarwidget) (`SceneComponent.K2_GetComponentLocation` (`PlayerCameraManager.TransformComponent` (`GameplayStatics.GetPlayerCameraManager` 0)))) false false))

(event `self.TowerRange.OnComponentBeginOverlap`
  (params (OverlappedComponent :type "PrimitiveComponent Object Reference") (OtherActor :type "Actor Object Reference") (OtherComp :type "PrimitiveComponent Object Reference") (OtherBodyIndex :type Integer) (bFromSweep :type Boolean) (SweepResult :type "HitResult Structure (by ref)"))
  ;[1 1 1] Detect if player are in range
  (cast `/Game/Blueprints/Characters/BP_Hero` OtherActor)
  (bind _returnvalue (`KismetSystemLibrary.K2_SetTimerDelegate` (delegate `TowerAttack`) (`self.AttackSpeed`) true))
  (set `self.AttackTimer` _returnvalue))

(event `self.TowerRange.OnComponentEndOverlap`
  (params (OverlappedComponent :type "PrimitiveComponent Object Reference") (OtherActor :type "Actor Object Reference") (OtherComp :type "PrimitiveComponent Object Reference") (OtherBodyIndex :type Integer))
  ;[1 1 1] Detect if player are in range
  (cast `/Game/Blueprints/Characters/BP_Hero` OtherActor)
  (`KismetSystemLibrary.K2_ClearAndInvalidateTimerHandle` (`self.AttackTimer`)))

(event `TowerAttack`
  ;[1 1 1] Spawn projectile from tower
  (bind _returnvalue (`|SpawnActorFromClass` "/Game/Blueprints/Actors/BP_BigProjectile.BP_BigProjectile_C" (`SceneComponent.K2_GetComponentToWorld` (`self.Fire`)) "Undefined" "MultiplyWithRoot" null null))
  (`PrimitiveComponent.AddImpulse` (`/Game/Blueprints/Actors/BP_BigProjectile.Sphere` _returnvalue) (* (`KismetMathLibrary.GetDirectionUnitVector` (`self.K2_GetActorLocation` _returnvalue) (`self.K2_GetActorLocation` (`GameplayStatics.GetPlayerCharacter` 0))) 5000.0) "None" false))

(event `self.ReceiveAnyDamage`
  (params (Damage :type "Float (single-precision)") (DamageType :type "DamageType Object Reference") (InstigatedBy :type "Controller Object Reference") (DamageCauser :type "Actor Object Reference"))
  ;[1 1 1] Turret taking damage
  (bind _output_get (set `self.CurrentLife` (- (`self.CurrentLife`) Damage)))
  (`self.UpdateHealthBar`)
  (if (<= _output_get 0.0)
    (`self.K2_DestroyActor`)))

(fn `UpdateHealthBar`
  (bind _aswbp_tower_hud (cast `/Game/Blueprints/WidgetBlueprints/WBP_TowerHUD` (`WidgetComponent.GetWidget` (`self.HealthBarWidget`))))
  (`ProgressBar.SetPercent` (`/Game/Blueprints/WidgetBlueprints/WBP_TowerHUD.TowerHealthBar` _aswbp_tower_hud) (/ (`self.CurrentLife`) (`self.MaxLife`))))

(fn `UserConstructionScript`)