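; BP_SlowingBubble is a projectile actor that stops moving one second after spawn; despite its name, it applies no slowing effect.
; Every tick it draws a debug Camera-channel line trace from its Sphere to player 0's capsule, without using the result.
; A second sphere, Sphere1, only prints the names of actors that begin or end overlap with it.
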(event `self.ReceiveBeginPlay`
  (`KismetSystemLibrary.Delay` 1.0)
  (`MovementComponent.StopMovementImmediately` (`self.ProjectileMovement`)))

(event `self.ReceiveTick`
  (params (DeltaSeconds :type "Float (single-precision)"))
  (set `self.SelfLocation` (`SceneComponent.K2_GetComponentLocation` (`self.Sphere`)))
  (set `self.PlayerLocation` (`SceneComponent.K2_GetComponentLocation` (`Character.CapsuleComponent` (`GameplayStatics.GetPlayerCharacter` 0))))
  (`KismetSystemLibrary.LineTraceSingle` :`Start` (`self.SelfLocation`) :`End` (`self.PlayerLocation`) :`TraceChannel` "TraceTypeQuery2" :`DrawDebugType` "ForOneFrame" :`DrawTime` 1.0))

(event `self.Sphere1.OnComponentBeginOverlap`
  (params (OverlappedComponent :type "PrimitiveComponent Object Reference") (OtherActor :type "Actor Object Reference") (OtherComp :type "PrimitiveComponent Object Reference") (OtherBodyIndex :type Integer) (bFromSweep :type Boolean) (SweepResult :type "HitResult Structure (by ref)"))
  (`KismetSystemLibrary.PrintString` (`KismetSystemLibrary.GetDisplayName` OtherActor)))

(event `self.Sphere1.OnComponentEndOverlap`
  (params (OverlappedComponent :type "PrimitiveComponent Object Reference") (OtherActor :type "Actor Object Reference") (OtherComp :type "PrimitiveComponent Object Reference") (OtherBodyIndex :type Integer))
  (`KismetSystemLibrary.PrintString` (`KismetSystemLibrary.GetDisplayName` OtherActor)))

(fn `UserConstructionScript`)