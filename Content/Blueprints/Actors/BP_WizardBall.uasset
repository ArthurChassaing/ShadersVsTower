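; BP_WizardBall is a projectile actor, tied by name and stored reference to the wizard player, that damages towers.
; On BeginPlay it activates its particle effect and caches the player character as a BP_Wizard.
; Sphere hits ignore that character; a hit on a BP_Tower applies the projectile's damage and destroys the ball.
; Hits on any other actor neither deal damage nor destroy it.
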(event `self.ReceiveBeginPlay`
  (`ActorComponent.SetActive` (`self.Particles`) true true)
  (bind _asbp_wizard (cast `/Game/Blueprints/Characters/BP_Wizard` (`GameplayStatics.GetPlayerCharacter` 0)))
  (set `self.CharacterRef` _asbp_wizard))

(event `self.Sphere.OnComponentHit`
  (params (HitComponent :type "PrimitiveComponent Object Reference") (OtherActor :type "Actor Object Reference") (OtherComp :type "PrimitiveComponent Object Reference") (NormalImpulse :type "Vector Structure") (Hit :type "HitResult Structure (by ref)"))
  (if (!= OtherActor (`self.CharacterRef`))
    (bind _asbp_tower (cast `/Game/Blueprints/Actors/BP_Tower` OtherActor))
    (`GameplayStatics.ApplyDamage` _asbp_tower (`self.DamageProjectile`) null self)
    (`self.K2_DestroyActor`)))

(fn `UserConstructionScript`)