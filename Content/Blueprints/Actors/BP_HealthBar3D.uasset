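; BP_HealthBar3D is a world-space health bar actor that shows a health percentage and turns to face the player.
; On BeginPlay it caches the progress bar from the WB_HealthBar widget in its HealthBarCanvas component.
; UpdateHeathPercentage sets that bar to Health / MaxHealth, with the clamp node left unconnected.
; Every Tick, FacePlayer rotates the whole actor toward player pawn 0 using a look-at rotation.
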(event `self.ReceiveBeginPlay`
  ;[1 1 1] Init HealtBar Variable
  (bind _aswb_health_bar (cast `/Game/Blueprints/WidgetBlueprints/WB_HealthBar` (`WidgetComponent.GetWidget` (`self.HealthBarCanvas`))))
  (set `self.HealthProgressBar` (`/Game/Blueprints/WidgetBlueprints/WB_HealthBar.HealthProgressBar` _aswb_health_bar)))

(event `self.ReceiveTick`
  (params (DeltaSeconds :type "Float (single-precision)"))
  ;[1 1 1] Face the player every frame
  (`self.FacePlayer`))

(fn `FacePlayer`
  ;[1 1 1] Compute rotation between self and player, then rotate to face player
  (`self.K2_SetActorRotation` (`KismetMathLibrary.FindLookAtRotation` (`self.K2_GetActorLocation`) (`self.K2_GetActorLocation` (`GameplayStatics.GetPlayerPawn` 0)))))

(fn `UpdateHeathPercentage`
  (params (Health :type "Float (double-precision)") (MaxHealth :type "Float (double-precision)"))
  ;[1 1 1] Clamp the health and compute the percentage of health to be set
  (`ProgressBar.SetPercent` (`self.HealthProgressBar`) (/ Health MaxHealth)))

(fn `UserConstructionScript`)