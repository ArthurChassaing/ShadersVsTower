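; BP_Shadow is a short-lived shadow actor that shows an ash material on a poseable mesh, then removes itself.
; On BeginPlay it creates one dynamic instance of M_ShadowAsh and applies it to every material slot.
; A timeline then feeds a scalar parameter on that instance, though its name is left as None, and destroys the actor when finished.
; No pose is set within this Blueprint.
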(event `self.ReceiveBeginPlay`
  (`|ExecutionSequence`
    (:`then_0`
      (bind _returnvalue (`KismetMaterialLibrary.CreateDynamicMaterialInstance` "/Game/Art/Materials/M_ShadowAsh.M_ShadowAsh"))
      (bind _output_get (set `self.MaterialToCreate` _returnvalue))
      (for _index (range (`PrimitiveComponent.GetNumMaterials` (`self.PoseableMesh`)))
        (`PrimitiveComponent.SetMaterial` (`self.PoseableMesh`) _index _output_get)))
    (:`then_1`
      (bind (_direction _newtrack_0) (`Timeline|Timeline`)
        (:`Update`
          (`MaterialInstanceDynamic.SetScalarParameterValue` (`self.MaterialToCreate`) "None" _newtrack_0))
        (:`Finished`
          (`self.K2_DestroyActor`))))))

(fn `UserConstructionScript`)