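; Game mode for ShaderTower that swaps the player's character on request and provides a level-restarting game over.
; It listens to the shader controller's character-change event, spawns the indexed class at the current capsule transform, destroys the old pawn and possesses the new one.
; After each swap it updates the controller's player reference and rebinds the hero's death event.
; GameOver reloads the level through a console command.
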(event `self.ReceiveBeginPlay`
  (bind _asbp_shader_controller (cast `/Game/Blueprints/Controllers/BP_ShaderController` (`GameplayStatics.GetPlayerController` 0)))
  (set `self.Shader Controller` _asbp_shader_controller)
  (add `/Game/Blueprints/Controllers/BP_ShaderController.OnCharacterChange` _asbp_shader_controller (delegate `OnCharacterChange_Event`))
  (bind _asbp_hero (cast `/Game/Blueprints/Characters/BP_Hero` (`GameplayStatics.GetPlayerCharacter` 0) :!label _label))
  (add `/Game/Blueprints/Characters/BP_Hero.OnDie` _asbp_hero (`|CreateDelegate` :!event `GameOver`)))

(event `OnCharacterChange_Event`
  (params (number :type Integer))
  (`self.ChangeCharacter` number)
  (goto _label))

(fn `ChangeCharacter`
  (params (Int :type Integer))
  (bind _returnvalue (`GameplayStatics.GetPlayerCharacter` 0))
  (bind _shader_controller (`self.Shader Controller`))
  (bind _returnvalue_2 (`|SpawnActorFromClass` (`|GetArrayItem` (`self.Characters`) Int) (`SceneComponent.K2_GetComponentToWorld` (`Character.CapsuleComponent` (`GameplayStatics.GetPlayerCharacter` 0))) "AlwaysSpawn" "MultiplyWithRoot" null null))
  (`self.K2_DestroyActor` _returnvalue)
  (`Controller.Possess` _shader_controller _returnvalue_2)
  (`/Game/Blueprints/Controllers/BP_ShaderController.SetPlayerRef` _shader_controller _returnvalue))

(fn `GameOver`
  (`KismetSystemLibrary.ExecuteConsoleCommand` "RestartLevel" null))

(fn `UserConstructionScript`)