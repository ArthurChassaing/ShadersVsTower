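; BP_Wizard is a wizard character Blueprint whose skill fires a magic ball projectile.
; OnSkillActivate runs the parent logic, then calls ShootProjectile, which flags the wizard as attacking.
; ShootProjectile spawns a scaled-down BP_WizardBall at the ProjectileSpawn transform and launches it with a physics impulse along that component's forward vector.
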(event `self.ReceiveBeginPlay`
  (`parent.ReceiveBeginPlay`))

(fn `OnSkillActivate`
  (`parent.OnSkillActivate`)
  (`self.ShootProjectile`))

(fn `ShootProjectile`
  (bind (_returnvalue_location _returnvalue_rotation) (`KismetMathLibrary.BreakTransform` (`SceneComponent.K2_GetComponentToWorld` (`self.ProjectileSpawn`))))
  (set `self.IsAttacking` true)
  (bind _returnvalue (`|SpawnActorFromClass` "/Game/Blueprints/Actors/BP_WizardBall.BP_WizardBall_C" (`KismetMathLibrary.MakeTransform` _returnvalue_location _returnvalue_rotation (0.1 0.1 0.1)) "AlwaysSpawn" "MultiplyWithRoot" null null))
  (`PrimitiveComponent.AddImpulse` (`/Game/Blueprints/Actors/BP_WizardBall.Sphere` _returnvalue) (* (`SceneComponent.GetForwardVector` (`self.ProjectileSpawn`)) 3000.0) "None" false))

(fn `UserConstructionScript`)