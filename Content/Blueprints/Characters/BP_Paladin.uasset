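; BP_Paladin is a playable hero character with a sword attack, a block and a self-heal skill.
; Enhanced Input toggles the blocking flag and plays the attack montage, which is locked against re-triggering until blend out.
; A Box overlap applies sword damage only to components tagged TowerMesh, without checking the attack state.
; The skill override calls its parent, then sets IsHealing and adds unclamped HealAmount to BP_Hero's CurrentLife.
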(event `EnhancedInput|/Game/Blueprints/InputActions/IA_Block`
  (params (ActionValue :type Boolean) (ElapsedSeconds :type "Float (double-precision)") (TriggeredSeconds :type "Float (double-precision)") (InputAction :type "InputAction Object Reference" :default "/Game/Blueprints/InputActions/IA_Block.IA_Block"))
  (:`Triggered`
    (set `self.IsBlocking` true))
  (:`Completed`
    (set `self.IsBlocking` false)))

(event `EnhancedInput|/Game/Blueprints/InputActions/IA_Attack`
  (params (ActionValue :type Boolean) (ElapsedSeconds :type "Float (double-precision)") (TriggeredSeconds :type "Float (double-precision)") (InputAction :type "InputAction Object Reference" :default "/Game/Blueprints/InputActions/IA_Attack.IA_Attack"))
  (:`Triggered`
    (if (not (`self.IsAttacking`))
      (`|PlayMontage` (`self.Mesh`) "/Game/Art/Anim/DefaultAttack_AnimMontage.DefaultAttack_AnimMontage" 1.2
        (:`then`
          (set `self.IsAttacking` true))
        (:`OnBlendOut`
          (set `self.IsAttacking` false))))))

(event `self.Box.OnComponentBeginOverlap`
  (params (OverlappedComponent :type "PrimitiveComponent Object Reference") (OtherActor :type "Actor Object Reference") (OtherComp :type "PrimitiveComponent Object Reference") (OtherBodyIndex :type Integer) (bFromSweep :type Boolean) (SweepResult :type "HitResult Structure (by ref)"))
  (if (`ActorComponent.ComponentHasTag` OtherComp "TowerMesh")
    (`GameplayStatics.ApplyDamage` OtherActor (`self.Sword Damage`) null self)))

(fn `Heal`
  (set `self.IsHealing` true)
  (bind _asbp_hero (cast `/Game/Blueprints/Characters/BP_Hero` self))
  (set `/Game/Blueprints/Characters/BP_Hero.CurrentLife` (+ (`/Game/Blueprints/Characters/BP_Hero.CurrentLife` _asbp_hero) (`self.HealAmount`)) _asbp_hero))

(fn `OnSkillActivate`
  (`parent.OnSkillActivate`)
  (`self.Heal`))

(fn `UserConstructionScript`)