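; BP_Hero is the hero character Blueprint, handling the hero's life, damage and death notification.
; On BeginPlay it fills CurrentLife from MaxLife and adds a WBP_HeroHUD widget for player 0 to the viewport.
; AnyDamage subtracts from CurrentLife and calls OnDie once life reaches zero or below, with no guard against repeat calls.
; OnSkillActivate, Tick and the construction script are empty.
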(event `self.ReceiveBeginPlay`
  (set `self.CurrentLife` (`self.MaxLife`))
  (bind _returnvalue (`|CreateWidget` "/Game/Blueprints/Characters/WBP_HeroHUD.WBP_HeroHUD_C" (`GameplayStatics.GetPlayerController` 0)))
  (`UserWidget.AddToViewport` _returnvalue 0))

(event `self.ReceiveTick`
  (params (DeltaSeconds :type "Float (single-precision)")))

(event `self.ReceiveAnyDamage`
  (params (Damage :type "Float (single-precision)") (DamageType :type "DamageType Object Reference") (InstigatedBy :type "Controller Object Reference") (DamageCauser :type "Actor Object Reference"))
  (bind _output_get (set `self.CurrentLife` (- (`self.CurrentLife`) Damage)))
  (if (<= _output_get 0.0)
    (`self.OnDie`)))

(fn `OnSkillActivate`)

(fn `UserConstructionScript`)