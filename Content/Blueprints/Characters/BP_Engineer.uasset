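; BP_Engineer is a character Blueprint whose skill deploys a temporary shield attached to itself.
; OnSkillActivate runs the parent logic, spawns an enlarged BP_Shield at the engineer's transform, gives it a configurable lifespan and attaches it to the engineer.
; When the engineer is destroyed, it also destroys every directly attached actor, so any active shield goes with it.
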(event `self.ReceiveDestroyed`
  (for _array_element (`self.GetAttachedActors` true)
    (`self.K2_DestroyActor` _array_element)))

(fn `OnSkillActivate`
  (locals (AttachmentRule :type "EAttachmentRule Enum" :default "SnapToTarget"))
  (bind (_returnvalue_location _returnvalue_rotation _returnvalue_scale) (`KismetMathLibrary.BreakTransform` (`self.GetTransform`)))
  (bind _attachmentrule (`local.AttachmentRule`))
  (`parent.OnSkillActivate`)
  (bind _returnvalue (`|SpawnActorFromClass` "/Game/Blueprints/Actors/BP_Shield.BP_Shield_C" (`KismetMathLibrary.MakeTransform` _returnvalue_location _returnvalue_rotation (* _returnvalue_scale 3)) "AlwaysSpawn" "MultiplyWithRoot" null null))
  (`self.SetLifeSpan` _returnvalue (`self.ShieldLifespan`))
  (`self.K2_AttachToActor` _returnvalue self "None" _attachmentrule _attachmentrule "KeepWorld" true))

(fn `UserConstructionScript`)