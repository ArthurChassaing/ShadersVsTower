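; Player controller that maps Enhanced Input to movement, look and combat actions on a cached character reference.
; Fire triggers BP_Hero's skill, attack plays a montage, and jump, block and fire set state flags.
; Dash launches the character forward while a looping timer and DoN spawn a limited trail of BP_Shadow actors.
; Number keys, with AZERTY equivalents, request character changes; setters allow replacing the character and mesh references.
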(event `self.ReceiveBeginPlay`
  (set `self.PlayerReference` (`GameplayStatics.GetPlayerCharacter` 0))
  (`EnhancedInputSubsystemInterface.AddMappingContext` (pcsubsystem `EnhancedInputLocalPlayerSubsystem` self) "/Game/Blueprints/InputActions/IMC_Shader.IMC_Shader" 0 (struct)))

(event `EnhancedInput|/Game/Blueprints/InputActions/IA_Right`
  (params (ActionValue :type Boolean) (ElapsedSeconds :type "Float (double-precision)") (TriggeredSeconds :type "Float (double-precision)") (InputAction :type "InputAction Object Reference" :default "/Game/Blueprints/InputActions/IA_Right.IA_Right"))
  (bind _playerreference (`self.PlayerReference`))
  (:`Triggered`
    (`Pawn.AddMovementInput` _playerreference (`self.GetActorRightVector` _playerreference) 1.0 false)))

(event `EnhancedInput|/Game/Blueprints/InputActions/IA_Forward`
  (params (ActionValue :type Boolean) (ElapsedSeconds :type "Float (double-precision)") (TriggeredSeconds :type "Float (double-precision)") (InputAction :type "InputAction Object Reference" :default "/Game/Blueprints/InputActions/IA_Forward.IA_Forward"))
  (bind _playerreference (`self.PlayerReference`))
  (:`Triggered`
    (`Pawn.AddMovementInput` _playerreference (`self.GetActorForwardVector` _playerreference) 1.0 false)))

(event `EnhancedInput|/Game/Blueprints/InputActions/IA_Left`
  (params (ActionValue :type Boolean) (ElapsedSeconds :type "Float (double-precision)") (TriggeredSeconds :type "Float (double-precision)") (InputAction :type "InputAction Object Reference" :default "/Game/Blueprints/InputActions/IA_Left.IA_Left"))
  (bind _playerreference (`self.PlayerReference`))
  (:`Triggered`
    (`Pawn.AddMovementInput` _playerreference (`self.GetActorRightVector` _playerreference) -1.0 false)))

(event `EnhancedInput|/Game/Blueprints/InputActions/IA_Back`
  (params (ActionValue :type Boolean) (ElapsedSeconds :type "Float (double-precision)") (TriggeredSeconds :type "Float (double-precision)") (InputAction :type "InputAction Object Reference" :default "/Game/Blueprints/InputActions/IA_Back.IA_Back"))
  (bind _playerreference (`self.PlayerReference`))
  (:`Triggered`
    (`Pawn.AddMovementInput` _playerreference (`self.GetActorForwardVector` _playerreference) -1.0 false)))

(event `EnhancedInput|/Game/Blueprints/InputActions/IA_LookAround`
  (params (ActionValue :type "Vector2D Structure") (ElapsedSeconds :type "Float (double-precision)") (TriggeredSeconds :type "Float (double-precision)") (InputAction :type "InputAction Object Reference" :default "/Game/Blueprints/InputActions/IA_LookAround.IA_LookAround"))
  (:`Triggered`
    (`self.AddYawInput` ActionValue_X)
    (`self.AddPitchInput` ActionValue_Y)))

(event `EnhancedInput|/Game/Blueprints/InputActions/IA_Fire`
  (params (ActionValue :type Boolean) (ElapsedSeconds :type "Float (double-precision)") (TriggeredSeconds :type "Float (double-precision)") (InputAction :type "InputAction Object Reference" :default "/Game/Blueprints/InputActions/IA_Fire.IA_Fire"))
  (:`Started`
    (bind _asbp_hero (cast `/Game/Blueprints/Characters/BP_Hero` (`self.PlayerReference`)))
    (`/Game/Blueprints/Characters/BP_Hero.OnSkillActivate` _asbp_hero)
    (set `self.IsASpell` true))
  (:`Canceled`
    (set `self.IsASpell` false)))

(event `EnhancedInput|/Game/Blueprints/InputActions/IA_Jump`
  (params (ActionValue :type Boolean) (ElapsedSeconds :type "Float (double-precision)") (TriggeredSeconds :type "Float (double-precision)") (InputAction :type "InputAction Object Reference" :default "/Game/Blueprints/InputActions/IA_Jump.IA_Jump"))
  (bind _charactermovement (`Character.CharacterMovement` (`self.PlayerReference`)))
  (bind _returnvalue (`SceneComponent.GetForwardVector` (`Actor.RootComponent` (`self.PlayerReference`))))
  (:`Triggered`
    (`Character.Jump` (`self.PlayerReference`))
    (set `self.IsJumping` true)
    (`CharacterMovementComponent.AddImpulse` _charactermovement _returnvalue true)
    (`PawnMovementComponent.AddInputVector` _charactermovement _returnvalue false))
  (:`Completed`
    (`Character.StopJumping` (`self.PlayerReference`))
    (set `self.IsJumping` false)))

(event `EnhancedInput|/Game/Blueprints/InputActions/IA_Block`
  (params (ActionValue :type Boolean) (ElapsedSeconds :type "Float (double-precision)") (TriggeredSeconds :type "Float (double-precision)") (InputAction :type "InputAction Object Reference" :default "/Game/Blueprints/InputActions/IA_Block.IA_Block"))
  (:`Triggered`
    (set `self.IsBlocking` true))
  (:`Canceled`
    (set `self.IsBlocking` false)))

(event `EnhancedInput|/Game/Blueprints/InputActions/IA_Attack`
  (params (ActionValue :type Boolean) (ElapsedSeconds :type "Float (double-precision)") (TriggeredSeconds :type "Float (double-precision)") (InputAction :type "InputAction Object Reference" :default "/Game/Blueprints/InputActions/IA_Attack.IA_Attack"))
  (:`Triggered`
    (if (not (`self.Is Attacking`))
      (`|PlayMontage` (`self.Skeletal Mesh`) "/Game/Art/Anim/DefaultAttack_AnimMontage.DefaultAttack_AnimMontage" 1.2
        (:`then`
          (set `self.Is Attacking` true))
        (:`OnInterrupted`
          (set `self.Is Attacking` false))))))

(event `CustomEvent`
  ;[1 1 1] Dash
  (bind _counter (`/Engine/EditorBlueprintResources/StandardMacros.Do N` 5 :!label _label)
    (:`Exit`
      (`|SpawnActorFromClass` "/Game/Blueprints/Actors/BP_Shadow.BP_Shadow_C" (`SceneComponent.K2_GetComponentToWorld` (`Character.Mesh` (`self.PlayerReference`))) "Undefined" "MultiplyWithRoot" null null)
      (if (== 5 _counter)
        (`KismetSystemLibrary.K2_ClearAndInvalidateTimerHandle` (stale `EnhancedInput|/Game/Blueprints/InputActions/IA_Dash` _returnvalue))))))

(event `EnhancedInput|/Game/Blueprints/InputActions/IA_Dash`
  (params (ActionValue :type Boolean) (ElapsedSeconds :type "Float (double-precision)") (TriggeredSeconds :type "Float (double-precision)") (InputAction :type "InputAction Object Reference" :default "/Game/Blueprints/InputActions/IA_Dash.IA_Dash"))
  ;[1 1 1] Dash
  (:`Started`
    (`Character.LaunchCharacter` (`self.PlayerReference`) (* (`self.GetActorForwardVector` (`self.PlayerReference`)) (`self.Force`)) true false)
    (bind _returnvalue (`KismetSystemLibrary.K2_SetTimerDelegate` (delegate `CustomEvent`) 0.1 true))
    (goto _label :!via `Reset`)))

(event `Key|One`
  (params (Key :type "Key Structure"))
  (:`Pressed`
    (bind _number (`self.SendCharacterNumber` 0 :!label _label_2))
    (`self.OnCharacterChange` _number)))

(event `Key|Ampersand`
  (params (Key :type "Key Structure"))
  (:`Pressed`
    (goto _label_2)))

(event `Key|Two`
  (params (Key :type "Key Structure"))
  (:`Pressed`
    (bind _number (`self.SendCharacterNumber` 1 :!label _label_3))
    (`self.OnCharacterChange` _number)))

(event `Key|E_AccentAigu`
  (params (Key :type "Key Structure"))
  (:`Pressed`
    (goto _label_3)))

(event `Key|Quote`
  (params (Key :type "Key Structure"))
  (:`Pressed`
    (bind _number (`self.SendCharacterNumber` 2 :!label _label_4))
    (`self.OnCharacterChange` _number)))

(event `Key|Three`
  (params (Key :type "Key Structure"))
  (:`Pressed`
    (goto _label_4)))

(fn `SendCharacterNumber`
  (params (Num :type Integer))
  (returns (Number :type Integer))
  (return Num))

(fn `SetPlayerRef`
  (params (NewReference :type "Character Object Reference"))
  (set `self.PlayerReference` NewReference))

(fn `SetSkeletalRef`
  (params (SkeletalRef :type "SkeletalMeshComponent Object Reference"))
  (set `self.Skeletal Mesh` SkeletalRef))

(fn `UserConstructionScript`)