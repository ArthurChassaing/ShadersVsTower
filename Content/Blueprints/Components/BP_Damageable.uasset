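; BP_Damageable is a component that tracks health and reports damage and death.
; Health starts at MaxHealth on BeginPlay, and the Damage function subtracts the given value from it.
; Each hit calls TakeDamage with the new and maximum health, then OnDie whenever health is at or below zero.
; Health is not clamped, and further hits after death call OnDie again.
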(event `self.ReceiveBeginPlay`
  ;[1 1 1] Initialization
  (set `self.Health` (`self.MaxHealth`)))

(fn `Damage`
  (params (value :type "Float (double-precision)"))
  (bind _output_get (set `self.Health` (- (`self.Health`) value)))
  (`self.TakeDamage` _output_get (`self.MaxHealth`))
  (if (<= _output_get 0.0)
    (`self.OnDie`)))